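; Collision component that detects attack hits by sweeping between two sockets on an assigned mesh.
; While collision is enabled, each tick runs a multi-sphere object trace between the start and end sockets, skipping an editable ignore list.
; Each newly hit actor is recorded and broadcast through OnHit, so it registers only once per activation.
; Enabling collision clears that record, and getters expose the current state.
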(event `self.ReceiveTick`
  (params (DeltaSeconds :type "Float (single-precision)"))
  (if (`self.bIsCollisionEnabled`)
    (`self.CollisionTrace`)))

(event `SetCollisionMesh`
  (params (MeshComponent :type "PrimitiveComponent Object Reference"))
  (set `self.CollisionMeshComponent` MeshComponent))

(event `EnableCollision`
  (`self.ClearHitActors`)
  (set `self.bIsCollisionEnabled` true))

(event `DisableCollision`
  (set `self.bIsCollisionEnabled` false))

(event `ClearHitActors`
  (`KismetArrayLibrary.Array_Clear` (`self.AlreadyHitActors`)))

(event `CollisionTrace`
  (bind _collisionmeshcomponent (`self.CollisionMeshComponent`))
  (bind _outhits (`KismetSystemLibrary.SphereTraceMultiForObjects` (`SceneComponent.GetSocketLocation` _collisionmeshcomponent (`self.StartSocketName`)) (`SceneComponent.GetSocketLocation` _collisionmeshcomponent (`self.EndSocketName`)) (`self.TraceRadius`) (`self.CollisionObjectTypes`) false (`self.ActorstoIgnore`) (`self.DrawDebugType`) true (struct :`R` 1.0 :`A` 1.0) (struct :`G` 1.0 :`A` 1.0) 3.0))
  (for _array_element _outhits
    (bind _output_get (set `self.LastHit` _array_element))
    (bind (_bblockinghit _binitialoverlap _time _distance _location _impactpoint _normal _impactnormal _physmat _hitactor) (`GameplayStatics.BreakHitResult` _output_get))
    (if (not (`KismetArrayLibrary.Array_Contains` (`self.AlreadyHitActors`) _hitactor))
      (bind _output_get_2 (set `self.HitActor` _hitactor))
      (`KismetArrayLibrary.Array_Add` (`self.AlreadyHitActors`) _output_get_2)
      (`self.OnHit` (`self.LastHit`)))))

(fn `AddActorToIgnore`
  (params (InActor :type "Actor Object Reference (by ref)"))
  (`KismetArrayLibrary.Array_AddUnique` (`self.ActorstoIgnore`) InActor))

(fn `GetActorToIgnore`
  (returns (ReturnValue :type "Array of Actor Object Reference"))
  (return (`self.ActorstoIgnore`)))

(fn `GetAlreadyHitActors`
  (returns (ReturnValue :type "Array of Actor Object Reference"))
  (return (`self.AlreadyHitActors`)))

(fn `GetCollisionMeshComponent`
  (returns (ReturnValue :type "PrimitiveComponent Object Reference"))
  (return (`self.CollisionMeshComponent`)))

(fn `GetIsCollisionEnabled`
  (returns (ReturnValue :type Boolean))
  (return (`self.bIsCollisionEnabled`)))

(fn `GetLastHit`
  (returns (ReturnValue :type "HitResult Structure"))
  (return (`self.LastHit`)))

(fn `RemoveActorToIgnore`
  (params (InActorToRemove :type "Actor Object Reference (by ref)"))
  (`KismetArrayLibrary.Array_RemoveItem` (`self.ActorstoIgnore`) InActorToRemove))